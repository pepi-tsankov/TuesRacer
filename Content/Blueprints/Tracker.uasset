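; Race tracker actor that runs a lap-based checkpoint race through the player controller.
; On BeginPlay it pushes lap count and medal and best times to the controller, numbers the checkpoints, binds their cleared events and activates the first.
; Each cleared checkpoint plays a sound, reveals the next one and sets the respawn transform.
; The final checkpoint updates the lap, and reaching max laps completes and restarts the race.
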(event Custom|ApplySetings
  (bind _controlerreference (Variables|Default|GetControlerReference))
  ;[1 1 1] applyUserSetingsWhenGameStart
  (Variables|/Game/Blueprints/myPlayerControler.myPlayerControler_C|SetmaxLaps _controlerreference (Variables|CustomSetings|GetMaxLaps))
  (CallFunction|UpdateTimes)
  (Default|StartGameSetup _controlerreference))

(event Custom|CheckpointCleared
  (params (NextCheckpoint :type Integer))
  (bind _controlerreference (Variables|Default|GetControlerReference))
  ;[1 1 1] checkpointClearedCheck and restart race if nesessary
  (CallFunction|LapCheck NextCheckpoint)
  (Audio|Components|Audio|Play (Variables|/Script/Engine.AmbientSound|GetAudioComponent (Variables|CustomSetings|GetCheckpointSoundEffects)) 0.0)
  (if (Variables|/Game/Blueprints/myPlayerControler.myPlayerControler_C|GetRaceComplete _controlerreference)
    (Default|Restart _controlerreference)))

(event Custom|StartSequence
  (bind _checkpoint (Variables|Checkpoints|GetCheckpoint))
  ;[1 1 1] StartSequence/getAllcheckpoints and act first checkpoint and binds event
  (for (_array_element _array_index) (Variables|Checkpoints|GetCheckpoint)
    (Variables|/Game/Blueprints/Checkpoint.Checkpoint_C|SetCheckpointNumber _array_element (+ _array_index 1))
    (Variables|Default|SetTotalCheckpoints (Utilities|Array|Length _checkpoint))
    (CallFunction|ActivateCheckpoint (Utilities|Array|Get(acopy) _checkpoint))
    (for _array_element_2 (Variables|Checkpoints|GetCheckpoint)
      (EventDispatchers|AssignCheckpointCleared _array_element_2 (delegate Custom|CheckpointCleared))
      (Audio|Components|Audio|Play (Variables|/Script/Engine.AmbientSound|GetAudioComponent (Variables|CustomSetings|GetLevelMusic)) 0.0))))

(event EventBeginPlay
  ;[1 1 1] EventBeginPlay
  (bind _asmy_player_controler (Utilities|Casting|CastTomyPlayerControler (Game|GetPlayerController 0)))
  (Variables|Default|SetControlerReference _asmy_player_controler)
  (CallFunction|ApplySetings)
  (CallFunction|StartSequence))

(fn ConstructionScript)

(fn UpdateTimes
  (bind _controlerreference (Variables|Default|GetControlerReference))
  ;[1 1 1] Pass UserTimes to MPC times
  (Variables|/Game/Blueprints/myPlayerControler.myPlayerControler_C|SetGoldTime _controlerreference (Variables|CustomSetings|GetGoldTime))
  (Variables|/Game/Blueprints/myPlayerControler.myPlayerControler_C|SetSilverTime _controlerreference (Variables|CustomSetings|GetSilverTime))
  (Variables|/Game/Blueprints/myPlayerControler.myPlayerControler_C|SetBronzeTime _controlerreference (Variables|CustomSetings|GetBronzeTime))
  (Variables|/Game/Blueprints/myPlayerControler.myPlayerControler_C|SetDefaultBestRaceTime _controlerreference (Variables|CustomSetings|GetDefaultBestTime))
  (Variables|/Game/Blueprints/myPlayerControler.myPlayerControler_C|SetDefaultBestLapTime _controlerreference (Variables|CustomSetings|GetDefaultBestLap)))

(fn LapCheck
  (params (Checkpoint :type Integer))
  ;[1 1 1] LapCheckScript
  (bind _output_get (LocalVariables|SetLocalCheckpoint Checkpoint))
  (if (== _output_get (Variables|Default|GetTotalCheckpoints))
    (bind _isracecomplete_ (CallFunction|RaceCompleteCheck))
    (if _isracecomplete_
      _
      (else
        (CallFunction|ActivateCheckpoint (Utilities|Array|Get(acopy) (Variables|Checkpoints|GetCheckpoint)))))
    (Default|UpdateLap (Variables|Default|GetControlerReference))
    (else
      (CallFunction|ActivateCheckpoint (Utilities|Array|Get(acopy) (Variables|Checkpoints|GetCheckpoint) (LocalVariables|GetLocalCheckpoint)))))
  (Variables|/Game/Blueprints/myPlayerControler.myPlayerControler_C|SetRespawnLocation (Variables|Default|GetControlerReference) (Transformation|GetActorTransform (Utilities|Array|Get(acopy) (Variables|Checkpoints|GetCheckpoint) (- (LocalVariables|GetLocalCheckpoint) 1)))))

(fn ActivateCheckpoint
  (params (NextCheckpoint :type Checkpoint%20Object%20Reference))
  (bind _trigger (Variables|/Game/Blueprints/Checkpoint.Checkpoint_C|GetTrigger NextCheckpoint))
  ;[1 1 1] ActivateCheckpoint
  (Development|SetHiddeninGame _trigger false false)
  (Variables|/Script/Engine.PrimitiveComponent|SetbGenerateOverlapEvents _trigger true))

(fn RaceCompleteCheck
  (bind _controlerreference (Variables|Default|GetControlerReference))
  (bind _controlerreference_2 (Variables|Default|GetControlerReference))
  ;[1 1 1] RaceCompleteCheck
  (if (>= (Variables|/Game/Blueprints/myPlayerControler.myPlayerControler_C|GetactualLaps _controlerreference) (Variables|/Game/Blueprints/myPlayerControler.myPlayerControler_C|GetmaxLaps _controlerreference))
    (bind _output_get (Variables|/Game/Blueprints/myPlayerControler.myPlayerControler_C|SetRaceComplete _controlerreference_2 true))
    (LocalVariables|SetLocalComplete _output_get)
    (else
      (bind _output_get_2 (Variables|/Game/Blueprints/myPlayerControler.myPlayerControler_C|SetRaceComplete _controlerreference_2 false))
      (LocalVariables|SetLocalComplete _output_get_2)))
  (return (LocalVariables|GetLocalComplete)))