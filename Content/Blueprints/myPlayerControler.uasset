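; Player controller for a vehicle racing game that creates the HUD, runs race and lap timing, and handles vehicle respawning.
; BeginPlay caches the HUD and vehicle, then starts the GameTime timeline, which formats and prints elapsed race time.
; A separate LapTime timeline times laps, UpdateLap advances the count until the race completes, and RespawnVehicle spawns and possesses a new vehicle.
; Save/load, time checks, goal updates, setup and restart are empty stubs.
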(event Custom|StartGameSetup)

(event Custom|RespawnVehicle
  ;[1 1 1] respawn Vehicle
  (bind _returnvalue (Game|SpawnActorfromClass "/Game/VehicleAdvBP/Blueprints/VehicleBlueprint.VehicleBlueprint_C" (Variables|Default|GetRespawnLocation) "Undefined" 0 0))
  (Pawn|Possess _returnvalue))

(event Custom|StartRaceTime
  ;[1 1 1] Race/lap Timers
  (bind _time (Timeline|GameTime Play)
    (:Update
      (bind _output_get (Variables|ValueVariables|SetactualRaceTime _time))
      (bind _output_get_2 (Variables|TextVariables|SetRaceTimeText (Utilities|TimetoText _output_get)))
      (CallFunction|UpdateGoals)
      (Development|PrintText _output_get_2))))

(event Custom|StopRaceTime
  ;[1 1 1] Race/lap Timers
  (bind _time (Timeline|GameTime Stop)
    (:Update
      (bind _output_get (Variables|ValueVariables|SetactualRaceTime _time))
      (bind _output_get_2 (Variables|TextVariables|SetRaceTimeText (Utilities|TimetoText _output_get)))
      (CallFunction|UpdateGoals)
      (Development|PrintText _output_get_2))))

(event Custom|Restart)

(event Custom|StartLapTime
  ;[1 1 1] Race/lap Timers
  (bind _time (Timeline|LapTime PlayFromStart)
    (:Update
      (Variables|ValueVariables|SetactualLapTime _time))))

(event Custom|StopLapTime
  ;[1 1 1] Race/lap Timers
  (bind _time (Timeline|LapTime Stop)
    (:Update
      (Variables|ValueVariables|SetactualLapTime _time))))

(event Custom|UpdateLap
  ;[1 1 1] update lap
  (if (Variables|Default|GetRaceComplete)
    _
    (else
      (bind _output_get (Variables|ValueVariables|SetactualLaps (+ (Variables|ValueVariables|GetactualLaps) 1)))
      (bind _output_get_2 (Variables|TextVariables|SetCurentLapText (Utilities|Text|ToText(Integer) _output_get)))))
  (CallFunction|LapTimeCheck)
  (Development|PrintText _output_get_2))

(event EventBeginPlay
  ;[1 1 1] EventBeginPlay/getReferences
  (bind _returnvalue (UserInterface|CreateWidget "/Game/Blueprints/UI/HUD.HUD_C"))
  (bind _output_get (Variables|Default|SetHudReference _returnvalue))
  (UserInterface|Viewport|AddtoViewport _output_get 0)
  (bind _asvehicle_blueprint (Utilities|Casting|CastToVehicleBlueprint (Game|Player|GetPlayerPawn 0)))
  (Variables|Default|SetVehicleReference _asvehicle_blueprint)
  (CallFunction|StartRaceTime))

(fn ConstructionScript)

(fn InitText)

(fn SaveGameCheck)

(fn SaveGame)

(fn LoadGame)

(fn LapTimeCheck)

(fn RaceTimeCheck)

(fn UpdateGoals)